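; Tunnel generator that scrolls a chain of segment actors backward while the top-down controller's IsRunning is true, creating a moving-tunnel effect.
; BeginPlay spawns the initial segments in SequenceData order, snapping each to the previous segment's Forward component transform.
; Tick offsets segments against their Forward vector, then destroys the oldest once its world X drops below DestroyDistance and spawns the next.
; CurrentIndex only increments, with no wrap at the sequence end.
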(event EventBeginPlay
  ;[0.15 0.15 0.15 0.5] Get Player Controller and Spawn initial segments
  (bind _asbp_top_down_controller (Utilities|Casting|CastToBP_TopDownController (Game|GetPlayerController 0)))
  (Variables|Default|SetAs%20BP%20Top%20Down%20Controller _asbp_top_down_controller)
  (for _index (range 0 (Variables|Default|GetMaxSegments))
    (CallFunction|SpawnSegment)))

(event EventTick
  (params (DeltaSeconds :type Float%20%28single-precision%29))
  ;[0.15 0.15 0.15 0.5] Spawn Tunnel Segments adn move them
  (bind _output_get (Variables|Default|SetIs%20Running (Variables|/Game/TopDown/Blueprints/BP_TopDownController.BP_TopDownController_C|GetIsRunning (Variables|Default|GetAs%20BP%20Top%20Down%20Controller))))
  (if _output_get
    (for _array_element (Variables|Default|GetActiveSegments)
      (Transformation|AddActorWorldOffset _array_element (* (Variables|Default|Getspeed) DeltaSeconds (Math|Vector|GetForwardVector (Variables|/Game/BluePrints/LVL1_TunnelSegments/BP_TunnelSeg.BP_TunnelSeg_C|GetForward _array_element)) "-1.000000,-1.000000,-1.000000")))
    ;[0.15 0.15 0.15 0.5] Remove old segments
    (Math|Float|CompareFloat (.X (Math|Vector|BreakVector (Transformation|GetActorLocation (Utilities|Array|Get(acopy) (Variables|Default|GetActiveSegments))))) (Variables|Default|GetDestroyDistance)
      (:<
        (Actor|DestroyActor (Utilities|Array|Get(acopy) (Variables|Default|GetActiveSegments)))
        (Utilities|Array|RemoveIndex (Variables|Default|GetActiveSegments))
        (CallFunction|SpawnSegment)))))

(fn ConstructionScript)

(fn SpawnSegment
  (bind _output_get (Variables|Default|SetEntry (Utilities|Array|Get(acopy) (Variables|/Game/BluePrints/DA_Sequence.DA_Sequence_C|GetSegments (Variables|Default|GetSequenceData)) (Variables|Default|GetCurrentIndex))))
  (bind _returnvalue (Game|SpawnActorfromClass (Utilities|Struct|BreakST_Segmets _output_get) (Transformation|GetActorTransform) "Undefined" "MultiplyWithRoot" 0 0))
  (bind _output_get_2 (Variables|Default|SetNewSegment _returnvalue))
  (if (Utilities|IsValid (Variables|Default|GetLastSegment))
    (Transformation|SetActorTransform _output_get_2 (Transformation|GetWorldTransform (Variables|/Game/BluePrints/LVL1_TunnelSegments/BP_TunnelSeg.BP_TunnelSeg_C|GetForward (Variables|Default|GetLastSegment))))
    (Development|PrintString (Utilities|GetDisplayName (Variables|Default|GetLastSegment)))
    (else
      (Transformation|SetActorTransform _output_get_2 (Transformation|GetActorTransform))))
  (Utilities|Array|Add (Variables|Default|GetActiveSegments) _output_get_2)
  (Variables|Default|SetLastSegment _output_get_2)
  (Math|Integer|IncrementInt (Variables|Default|GetCurrentIndex)))