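; BP_TunnelSeg22 is a level 2 tunnel segment Blueprint with a moving laser hazard.
; Each Tick calls the parent, then offsets Laser along its right vector by a sine of time since creation, scaled by speed and distance, to move it up and down.
; The swept offset is per-frame without DeltaSeconds scaling, and feeds a world-space vector into a local-space move.
; It adds no overlap or construction logic of its own.
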(event EventBeginPlay
  (|CallParentFunction) ; This node is disabled and will not be called.\nDrag off pins to build functionality.
)

(event Collision|EventActorBeginOverlap
  (params (OtherActor :type Actor%20Object%20Reference))
  (|CallParentFunction OtherActor) ; This node is disabled and will not be called.\nDrag off pins to build functionality.
)

(event EventTick
  (params (DeltaSeconds :type Float%20%28single-precision%29))
  ;[0.15 0.15 0.15 0.5] Move Lasers up and Down
  (|CallParentFunction DeltaSeconds)
  (Transformation|AddLocalOffset (Variables|Default|GetLaser) (* (Math|Vector|GetRightVector (Variables|Default|GetLaser)) (* (Variables|Default|GetlaserSpeed) (* (Math|Trig|Sin(Radians) (Actor|GetGameTimeSinceCreation)) (Variables|Default|GetLaserDistance)))) true false))

(fn ConstructionScript
  (|CallParentFunction))