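; BP_TunnelSeg23 is a level 2 tunnel segment with a laser that moves back and forth.
; Each Tick calls the parent, then offsets the Laser component by its right vector times LaserSpeed, LaserDistance and the sine of time since creation.
; The swept offset accumulates per frame without delta-time scaling, so travel depends on frame rate, and it feeds a world-space vector into a local-space offset.
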(event EventBeginPlay
  (|CallParentFunction) ; This node is disabled and will not be called.\nDrag off pins to build functionality.
)

(event Collision|EventActorBeginOverlap
  (params (OtherActor :type Actor%20Object%20Reference))
  (|CallParentFunction OtherActor) ; This node is disabled and will not be called.\nDrag off pins to build functionality.
)

(event EventTick
  (params (DeltaSeconds :type Float%20%28single-precision%29))
  (|CallParentFunction DeltaSeconds)
  (Transformation|AddLocalOffset (Variables|Default|GetLaser) (* (Math|Vector|GetRightVector (Variables|Default|GetLaser)) (* (Variables|Default|GetLaser%20Speed) (* (Math|Trig|Sin(Radians) (Actor|GetGameTimeSinceCreation)) (Variables|Default|GetLaser%20Distance)))) true false))

(fn ConstructionScript
  (|CallParentFunction))